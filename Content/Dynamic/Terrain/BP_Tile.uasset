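; Terrain tile for an infinite-terrain game, with a collision barrier, trigger volumes and an arrow marking the attach transform.
; On BeginPlay it locks the barrier and calls PlaceActors.
; Player entry into the locking trigger turns the barrier green and passable; exit turns it red and solid and asks InfiniteTerrainGameMode to spawn a tile.
; Player overlap with the destroy trigger removes the tile.
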(event `self.ReceiveBeginPlay`
  (`self.Lock Level`)
  (`self.PlaceActors`))

(event `self.Locking_TriggerVolume.OnComponentBeginOverlap`
  (params (OverlappedComponent :type "PrimitiveComponent Object Reference") (OtherActor :type "Actor Object Reference") (OtherComp :type "PrimitiveComponent Object Reference") (OtherBodyIndex :type Integer) (bFromSweep :type Boolean) (SweepResult :type "HitResult Structure (by ref)"))
  (`self.Is Player Actor` OtherActor)
  (`self.Unlock Level`))

(event `self.Locking_TriggerVolume.OnComponentEndOverlap`
  (params (OverlappedComponent :type "PrimitiveComponent Object Reference") (OtherActor :type "Actor Object Reference") (OtherComp :type "PrimitiveComponent Object Reference") (OtherBodyIndex :type Integer))
  (`self.Is Player Actor` OtherActor)
  (`self.Lock Level`)
  (bind _asinfinite_terrain_game_mode (cast `/Game/Dynamic/InfiniteTerrainGameMode` (`GameplayStatics.GetGameMode`)))
  (`/Game/Dynamic/InfiniteTerrainGameMode.Spawn Tile` _asinfinite_terrain_game_mode))

(event `self.Destroy_TriggerVolume.OnComponentBeginOverlap`
  (params (OverlappedComponent :type "PrimitiveComponent Object Reference") (OtherActor :type "Actor Object Reference") (OtherComp :type "PrimitiveComponent Object Reference") (OtherBodyIndex :type Integer) (bFromSweep :type Boolean) (SweepResult :type "HitResult Structure (by ref)"))
  (`self.Is Player Actor` OtherActor)
  (`self.K2_DestroyActor`))

(fn `Get Attach Location`
  (returns (`Attach Transform` :type "Transform Structure"))
  (locals (`Barrier Open` :type Boolean))
  (return (`SceneComponent.K2_GetComponentToWorld` (`self.Arrow`))))

(fn `Lock Level`
  (`PrimitiveComponent.SetCollisionEnabled` (`self.Barrier`) "QueryAndPhysics")
  (`PrimitiveComponent.SetMaterial` (`self.Barrier`) 0 "/Game/Dynamic/Terrain/MI_Barrier_Red.MI_Barrier_Red"))

(fn `Unlock Level`
  (`PrimitiveComponent.SetCollisionEnabled` (`self.Barrier`) "NoCollision")
  (`PrimitiveComponent.SetMaterial` (`self.Barrier`) 0 "/Game/Dynamic/Terrain/MI_Barrier_Green.MI_Barrier_Green"))

(fn `UserConstructionScript`)